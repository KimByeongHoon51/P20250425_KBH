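; Player state Blueprint for a Vampire Survivors-style game that tracks the player's health and death.
; AddDamage ignores hits once IsDeath reports zero or lower HP; otherwise it subtracts damage from CurHp and broadcasts UpdateHp with current and max HP.
; It then fires the Death dispatcher when HP runs out, leaving responses to listeners.
; The event graph and construction script contain no logic.
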(fn `AddDamage`
  (params (Damage :type "Float (double-precision)"))
  (if (not (`self.IsDeath`))
    (bind _output_get (set `self.CurHp` (- (`self.CurHp`) Damage)))
    (`self.EventDispatcher_UpdateHp` _output_get (`self.MaxHp`))
    (if (<= (`self.CurHp`) 0.0)
      (`self.EventDispatcher_Death`))))

(fn `IsDeath`
  (returns (IsDeath :type Boolean))
  (return (<= (`self.CurHp`) 0.0)))

(fn `UserConstructionScript`)